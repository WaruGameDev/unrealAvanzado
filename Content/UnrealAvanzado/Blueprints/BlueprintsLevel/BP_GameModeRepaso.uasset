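; BP_GameModeRepaso is a game mode for a marble level that runs an elapsed-time timer and handles checkpoint respawns.
; BeginPlay stores the player pawn's location as the first checkpoint, then creates the WBP_TimerUI widget and starts timing.
; Tick accumulates elapsed time and pushes it to the widget.
; SetCheckPoint replaces the stored position, and Respawn teleports the BP_Marble pawn back to it.
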(event `self.ReceiveTick`
  (params (DeltaSeconds :type "Float (single-precision)"))
  (if (`self.RunningTime`)
    (bind _output_get (set `self.ElapsedTime` (+ (`self.ElapsedTime`) DeltaSeconds)))
    (bind _uitimer (`self.UITimer`)
      (:`then`
        (`/Game/UnrealAvanzado/Blueprints/UI/WBP_TimerUI.ShowUITimer` _uitimer _output_get))
      (:`else`))))

(event `self.ReceiveBeginPlay`
  (set `self.LastCheckPointPosition` (`self.K2_GetActorLocation` (`GameplayStatics.GetPlayerPawn` 0)))
  (`self.StartTimer`))

(fn `Respawn`
  (bind _asbp_marble (cast `/Game/UnrealAvanzado/Blueprints/BP_Marble` (`GameplayStatics.GetPlayerPawn` 0)))
  (`/Game/UnrealAvanzado/Blueprints/BP_Marble.Teleport` _asbp_marble (`self.LastCheckPointPosition`)))

(fn `SetCheckPoint`
  (params (LastCheckPointPosition :type "Vector Structure"))
  (set `self.LastCheckPointPosition` LastCheckPointPosition))

(fn `StartTimer`
  (bind _returnvalue (`|CreateWidget` "/Game/UnrealAvanzado/Blueprints/UI/WBP_TimerUI.WBP_TimerUI_C"))
  (bind _output_get (set `self.UITimer` _returnvalue))
  (`UserWidget.AddToViewport` _output_get 0)
  (set `self.RunningTime` true))

(fn `UserConstructionScript`)